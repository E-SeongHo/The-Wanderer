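; BP_Wanderer is the Wanderer character Blueprint, adding debug visuals and hard-wired test keys to a character with a combat component.
; R toggles between CombatCam and the default camera, Q plays an execution montage, and 0 ragdolls the mesh.
; Tick draws debug arrows for forward, right and horizontal velocity direction.
; Combat-target debug drawing and camera animation nodes are left unconnected.
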(event EventBeginPlay)

(event Collision|EventActorBeginOverlap
  (params (OtherActor :type Actor%20Object%20Reference)))

(event EventTick
  (params (DeltaSeconds :type Float%20%28single-precision%29))
  (Rendering|Debug|DrawDebugArrow (Transformation|GetActorLocation) (+ (Transformation|GetActorLocation) (* (Transformation|GetActorForwardVector) "100.000000,100.000000,100.000000")) 1e+01 "(R=0.340781,G=1.000000,B=0.356487,A=1.000000)" 0.0 1e+01)
  (Rendering|Debug|DrawDebugArrow (Transformation|GetActorLocation) (+ (Transformation|GetActorLocation) (* (Transformation|GetActorRightVector) "100.000000,100.000000,100.000000")) 1e+01 "(R=0.293738,G=1.000000,B=0.562024,A=1.000000)" 0.0 1e+01)
  (Rendering|Debug|DrawDebugArrow (Transformation|GetActorLocation) (+ (Transformation|GetActorLocation) (* (Class|KismetMathLibrary|VectorNormal2D (Transformation|GetVelocity) 0.0001) "100.000000,100.000000,100.000000")) 1e+01 "(R=1.000000,G=0.342494,B=0.322596,A=1.000000)" 0.0 1e+01))

(event Input|KeyboardEvents|R
  (params (Key :type Key%20Structure :default "None"))
  (bind _cameracomponent (Variables|Default|GetCameraComponent))
  (bind _combat_cam (Variables|Default|GetCombat%20Cam))
  (:Pressed
    (Utilities|FlowControl|FlipFlop
      (:A
        (Components|Activation|Activate _combat_cam false)
        (Components|Activation|Deactivate _cameracomponent))
      (:B
        (Components|Activation|Deactivate _combat_cam)
        (Components|Activation|Activate _cameracomponent false)))))

(event Input|KeyboardEvents|Q
  (params (Key :type Key%20Structure :default "None"))
  (:Pressed
    (Animation|Montage|PlayMontage (Variables|Character|GetMesh) "/Game/TheWanderer/Assets/Animations/Samurai/GhostSamurai_Execution02_Montage.GhostSamurai_Execution02_Montage")))

(event Input|KeyboardEvents|0
  (params (Key :type Key%20Structure :default "None"))
  (bind _mesh (Variables|Character|GetMesh))
  (:Pressed
    (Physics|SetSimulatePhysics _mesh true)
    (Collision|SetCollisionProfileName _mesh "Ragdoll" true :!class /Script/Engine.PrimitiveComponent)))

(fn ConstructionScript)